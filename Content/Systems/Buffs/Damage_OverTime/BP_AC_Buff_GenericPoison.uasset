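; Generic damage-over-time buff component for poison-style effects that damages its owning character's health on each buff tick, ignoring armor.
; Each tick sets the cause of death through the combat interface, then applies per-tick damage scaled exponentially by stack size (stack count raised to a configurable power).
; Instances tagged "Bleed" have their damage reduced when the owner carries a Hemostasis buff component.
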(event EventGameplayEffecttoApplyonBuffTick
  (bind _asis_base_bpcombat_interface (Utilities|Casting|CastToIsBaseBPCombatInterface (Variables|Default|GetOwningCharacter)))
  (Default|SetCauseOfDeath _asis_base_bpcombat_interface (Variables|Default|GetCauseOfDeath))
  (CallFunction|BuffApplyDamage (* (CallFunction|GetTickDamage) (CallFunction|GetPoisonDamageMultiplier)) "/Game/Systems/Progression/DmgTypeHealth_IgnoreArmor_BP.DmgTypeHealth_IgnoreArmor_BP_C"))

(fn GetTickDamage
  (return (* (Variables|Default|GetDamagePerBuffTick) (Math|Float|Power (Math|Conversions|ToFloat(Integer) (Variables|Default|GetStackSize)) (Variables|Default|GetDamageStackExp)))))

(fn GetPoisonDamageMultiplier
  (bind _owningcharacter (Variables|Default|GetOwningCharacter))
  (bind _returnvalue (Actor|GetComponentbyClass _owningcharacter "/Game/Mods/true-survival/Buffs/TS_Buff_Hemostasis.TS_Buff_Hemostasis_C"))
  (if (and (Components|ComponentHasTag "Bleed") (Utilities|IsValid _returnvalue))
    (return (- 1.0 (Variables|/Game/Mods/true-survival/Buffs/TS_Buff_Hemostasis.TS_Buff_Hemostasis_C|GetBleed%20Damage%20Reduction _returnvalue)))
    (else
      (return 1.0))))